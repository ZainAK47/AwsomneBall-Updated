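; BP_WinLevel_Box is a box trigger that completes the current level when the player pawn overlaps it.
; CompleteLevel looks up the current level's name in the LevelNames array and opens the next entry by name.
; When the current level is the last entry, it quits the game instead.
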(event OnComponentBeginOverlap(WinLevelTrigger_Box)
  (params (OverlappedComponent :type Primitive%20Component%20Object%20Reference) (OtherActor :type Actor%20Object%20Reference) (OtherComp :type Primitive%20Component%20Object%20Reference) (OtherBodyIndex :type Integer) (bFromSweep :type Boolean) (SweepResult :type Hit%20Result%20Structure%20%28by%20ref%29))
  (if (== OtherActor (Game|Player|GetPlayerPawn 0))
    (CallFunction|CompleteLevel)))

(event EventBeginPlay)

(event EventTick
  (params (DeltaSeconds :type Float%20%28single-precision%29)))

(fn ConstructionScript)

(fn CompleteLevel
  (bind _level_names (Variables|Default|GetLevel_Names))
  (bind _returnvalue (Game|GetCurrentLevelName true))
  (if (== (Utilities|Array|LastIndex _level_names) (Utilities|Array|FindItem _level_names (Utilities|String|StringToName _returnvalue)))
    (Game|QuitGame 0 "Quit" false)
    (else
      (Game|OpenLevel(byName) (Utilities|Array|Get(acopy) (Variables|Default|GetLevel_Names) (+ (Utilities|Array|FindItem _level_names (Utilities|String|StringToName _returnvalue)) 1))))))