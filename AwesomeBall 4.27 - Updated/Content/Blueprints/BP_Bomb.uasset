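; BP_Bomb is a hazard that knocks the ball pawn away and carries a negative point value.
; On BeginPlay it sets the point penalty and explosion sound and particle effect, then calls the parent.
; On overlap with BP_BallPawn, it applies a velocity-change radial impulse to the ball mesh from below the bomb's location, giving an upward kick, then hands off to the parent's overlap logic.
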(event EventBeginPlay
  (Variables|Default|SetNumOfPoints -5)
  (Variables|Default|SetThe_Sound "/Game/StarterContent/Audio/Explosion_Cue.Explosion_Cue")
  (Variables|Default|SetThe_Particle_System "/Game/StarterContent/Particles/P_Explosion.P_Explosion")
  (|CallParentFunction))

(event Collision|EventActorBeginOverlap
  (params (OtherActor :type Actor%20Object%20Reference))
  (|CallParentFunction OtherActor) ; This node is disabled and will not be called.\nDrag off pins to build functionality.
)

(event EventTick
  (params (DeltaSeconds :type Float%20%28single-precision%29))
  (|CallParentFunction DeltaSeconds) ; This node is disabled and will not be called.\nDrag off pins to build functionality.
)

(event EventOnOverlapped
  (params (Object :type Object%20Object%20Reference))
  (bind _returnvalue (Transformation|GetActorLocation))
  (bind _asbp_ball_pawn (Utilities|Casting|CastToBP_BallPawn Object))
  (Physics|AddRadialImpulse (Variables|/Game/Blueprints/BP_BallPawn.BP_BallPawn_C|GetBall_Mesh _asbp_ball_pawn) (Math|Vector|MakeVector (.x _returnvalue) (.y _returnvalue) (- (.z _returnvalue) 75.0)) 4e+02 1e+03 "RIF_Constant" true)
  (|CallParentFunction Object))

(fn ConstructionScript
  (|CallParentFunction))