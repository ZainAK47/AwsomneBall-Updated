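; BP_BallPawn is a torque-rolled player ball with hit-reset jumping and randomized material and scale.
; Tick drives a countdown that pauses into a Retry widget at zero, and feeds progress toward the EndGame actor to a position widget.
; Releasing Q destroys the player and inserts the score into loaded ScoreSave entries, but saving and scoreboard display are unwired.
; IncrementScore keeps SCORE non-negative, separate from the recorded NumOfPoints.
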(event OnComponentActivated(Camera)
  (params (Component :type Actor%20Component%20Object%20Reference) (bReset :type Boolean)))

(event Collision|EventActorBeginOverlap
  (params (OtherActor :type Actor%20Object%20Reference)))

(event Collision|EventHit
  (params (MyComp :type Primitive%20Component%20Object%20Reference) (Other :type Actor%20Object%20Reference) (OtherComp :type Primitive%20Component%20Object%20Reference) (bSelfMoved :type Boolean) (HitLocation :type Vector :default "0, 0, 0") (HitNormal :type Vector :default "0, 0, 0") (NormalImpulse :type Vector :default "0, 0, 0") (Hit :type Hit%20Result%20Structure%20%28by%20ref%29))
  ;[1 1 1] Handles Ball Jump
  (Variables|Default|SetCanBallJump true))

(event EventBeginPlay
  (bind _randballmaterial (Variables|Default|GetRandBallMaterial))
  (bind _randsize (Variables|Default|GetRandSize))
  (bind _returnvalue (Utilities|Array|LastIndex _randsize))
  (bind _returnvalue_2 (Math|Random|RandomIntegerinRange 0 _returnvalue))
  (bind _output (Utilities|Array|Get(acopy) _randsize _returnvalue_2))
  ;[1 1 1] Handles Random Balls Spawning
  (Utilities|FlowControl|Sequence
    (:then_0
      (Rendering|Material|SetMaterial (Variables|Default|GetBall_Mesh) 0 (Utilities|Array|Get(acopy) _randballmaterial (Math|Random|RandomIntegerinRange 0 (Utilities|Array|LastIndex _randballmaterial))))
      (Transformation|SetRelativeScale3D (Variables|Default|GetBall_Mesh) (Math|Vector|MakeVector _output _output _output))
      (Variables|Default|SetBallSpawnLocat (Transformation|GetActorLocation))
      (bind _returnvalue_3 (Actor|GetActorOfClass "/Game/Blueprints/EndGame.EndGame_C"))
      (Variables|Default|SetEndLocation (Transformation|GetActorLocation _returnvalue_3)))
    (:then_1
      ;[1 1 1] Displays Position Widget
      (bind _returnvalue_4 (UserInterface|CreateWidget "/Game/Blueprints/BP_Position.BP_Position_C"))
      (bind _output_get (Variables|Default|SetBp_Position%20Widget _returnvalue_4))
      (UserInterface|Viewport|AddtoViewport _output_get 0))))

(event EventTick
  (params (DeltaSeconds :type Float%20%28single-precision%29))
  ;[1 1 1] Handles Countdown Timer
  (Utilities|FlowControl|Sequence
    (:then_0
      (bind _output_get (Variables|Default|SetNewVar_0 (- (Variables|Default|Gettime_limt) (stale _output_get_3))))
      (Variables|Default|SetSeconds (Math|Float|Truncate (Math|Float|%(Float) _output_get 6e+01)))
      (Variables|Default|SetMinutes (Math|Float|Truncate (/ _output_get 6e+01)))
      (if (== (Math|Float|Truncate _output_get) 0)
        ;[1 1 1] Handles Retry functionality
        (bind _returnvalue (UserInterface|CreateWidget "/Game/Blueprints/Retry.Retry_C"))
        (UserInterface|Viewport|AddtoViewport _returnvalue 0)
        (Variables|/Script/Engine.PlayerController|SetbShowMouseCursor (Game|GetPlayerController 0) true)
        (Game|SetGamePaused true)))
    (:then_1
      ;[1 1 1] progress
      (bind _output_get_2 (Variables|Default|Setprogress (Math|Float|Clamp(Float) (* 100 (/ (Math|Vector|Distance(Vector) (Transformation|GetActorLocation) (Variables|Default|GetBallSpawnLocat)) (Math|Vector|Distance(Vector) "0, 0, 0" (Variables|Default|GetEndLocation)))) 0.0 1e+02)))
      (Variables|/Game/Blueprints/BP_Position.BP_Position_C|Setprogres (Variables|Default|GetBp_Position%20Widget) _output_get_2))
    (:then_2
      (bind _output_get_3 (Variables|Default|Settime (+ DeltaSeconds (Variables|Default|Gettime)))))))

(event Input|ActionEvents|InputActionJumping
  (params (Key :type Key%20Structure :default "None"))
  ;[1 1 1] Handles Ball Jump
  (:Pressed
    (if (Variables|Default|GetCanBallJump)
      (Physics|AddImpulse (Variables|Default|GetBall_Mesh) (Math|Vector|MakeVector 0.0 0.0 (Variables|Default|GetImpulseValue)) "None" true)
      (Variables|Default|SetCanBallJump false))))

(event Input|AxisEvents|InputAxisMoveForwards/Backwards
  (params (AxisValue :type Float%20%28single-precision%29))
  ;[1 1 1] Handles Ball Movement
  (Class|PrimitiveComponent|AddTorqueinRadians (Variables|Default|GetBall_Mesh) (Math|Vector|MakeVector 0.0 (* AxisValue (Variables|Default|GetSpeedFB)) 0.0) "None" true))

(event Input|AxisEvents|InputAxisMoveLeft?Right
  (params (AxisValue :type Float%20%28single-precision%29))
  ;[1 1 1] Handles Ball Movement
  (Class|PrimitiveComponent|AddTorqueinRadians (Variables|Default|GetBall_Mesh) (Math|Vector|MakeVector (* AxisValue (Variables|Default|GetSpeedLR)) 0.0 0.0) "None" true))

(event Input|KeyboardEvents|Q
  (params (Key :type Key%20Structure :default "None"))
  (bind _temp_array (Variables|Default|Gettemp_array))
  (bind _numofpoints (Variables|Default|GetNumOfPoints))
  (:Released
    (Utilities|FlowControl|DoOnce false
      (:Completed
        (Actor|DestroyActor (Game|GetPlayerCharacter 0))
        ;[1 1 1] Handling Score Board Functionality
        (bind _returnvalue (SaveGame|LoadGamefromSlot "ScoreSave"))
        (bind _asscore_save (Utilities|Casting|CastToScoreSave _returnvalue)
          (:then
            (for _array_element (Variables|/Game/Blueprints/ScoreSave.ScoreSave_C|GetPlayeScores _asscore_save)
              (Utilities|FlowControl|Sequence
                (:then_0
                  (if (<= (.Score (Utilities|Struct|BreakPlayerScore _array_element)) _numofpoints)
                    (Utilities|FlowControl|DoOnce false
                      (:Completed
                        (Utilities|Array|Add _temp_array (Utilities|Struct|MakePlayerScore "Player" _numofpoints (Class|KismetMathLibrary|GetDate)))))))
                (:then_1
                  (Utilities|Array|Add _temp_array _array_element))))
            (Utilities|FlowControl|Sequence
              (:then_0
                (Utilities|FlowControl|DoOnce false :!label _label
                  (:Completed
                    (Utilities|Array|Add _temp_array (Utilities|Struct|MakePlayerScore "Player" _numofpoints (Class|KismetMathLibrary|GetDate))))))
              (:then_1
                (bind _returnvalue_2 (SaveGame|CreateSaveGameObject "/Game/Blueprints/ScoreSave.ScoreSave_C" :!label _label_2))
                (bind _asscore_save_2 (Utilities|Casting|CastToScoreSave _returnvalue_2)))))
          (:CastFailed
            (Utilities|FlowControl|Sequence
              (:then_0
                (goto _label))
              (:then_1
                (goto _label_2)))))))))

(fn ConstructionScript)

(fn IncrementScore
  (params (In%20Score :type Integer))
  (if (< (+ In%20Score (Variables|Default|GetSCORE)) 0)
    (Variables|Default|SetSCORE 0)
    (else
      (Variables|Default|SetSCORE (+ In%20Score (Variables|Default|GetSCORE))))))